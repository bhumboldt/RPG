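; BP_WolfAI is a wolf AI character that moves toward enemies it sees.
; When PawnSensing sights a pawn that the Behavior component classifies as an enemy, it issues an AI Move To that stops within an acceptance radius.
; MeleeCollisionHandler activation for the Wolf part sets the body mesh and wolf sockets as the melee hit source.
; GetMontages supplies the wolf montage data table for any requested action.
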(event `self.ReceiveBeginPlay`
  (`parent.ReceiveBeginPlay`))

(event `self.MeleeCollisionHandler.OnCollisionActivated`
  (params (CollisionPart :type "/Game/DynamicCombatSystem/Enumerations/E_CollisionPart Enum" :default "NewEnumerator8"))
  (switch `/Game/DynamicCombatSystem/Enumerations/E_CollisionPart` CollisionPart
    (:`NewEnumerator9`
      ;[1 0 0] Body Part Collisions
      (`/Game/DynamicCombatSystem/Blueprints/Components/CollisionHandlerComponent.SetCollisionMesh` (`self.MeleeCollisionHandler`) (`self.Mesh`) (`self.WolfSocket`)))))

(event `self.PawnSensing.OnSeePawn`
  (params (Pawn :type "Pawn Object Reference"))
  (if (`/Game/DynamicCombatSystem/Blueprints/Components/BehaviorComponent.IsEnemy` (`self.Behavior`) Pawn)
    (`|AIMoveTo` self (0.0 0.0 0.0) Pawn 300.0)))

(fn `GetMontages`
  (params (Action :type "/Game/DynamicCombatSystem/Enumerations/E_MontageAction Enum" :default "NewEnumerator35"))
  (returns (Montages :type "DataTable Object Reference"))
  (return "/Game/AnimalVarietyPack/Wolf/DT_Wolf_Montages.DT_Wolf_Montages"))

(fn `UserConstructionScript`
  (`parent.UserConstructionScript`))